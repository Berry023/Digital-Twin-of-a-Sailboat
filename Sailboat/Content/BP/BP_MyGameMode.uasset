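; Game mode for a sailing game that spawns the fleet and hands the player a boat when play begins.
; It reads the boat count from BP_SailingGameInstance and spawns that many BP_Sailboat actors in an evenly spaced line along X, all sharing one heading.
; Spawned boats are stored in BoatArray, and the first player's SailboatControler possesses the first one.
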(event `self.ReceiveBeginPlay`
  (bind _asbp_sailing_game_instance (cast `/Game/BP/BP_SailingGameInstance` (`GameplayStatics.GetGameInstance`)))
  (for _index (range (`/Game/BP/BP_SailingGameInstance.BoatCount` _asbp_sailing_game_instance))
    (bind _returnvalue (`|SpawnActorFromClass` "/Game/BP/BP_Sailboat.BP_Sailboat_C" (`KismetMathLibrary.MakeTransform` (`KismetMathLibrary.MakeVector` (`KismetMathLibrary.Conv_IntToDouble` (+ (* _index -1000) -23000)) 15600.0 1200.0) (`KismetMathLibrary.MakeRotator` 0.0 0.0 90.0)) "Undefined" "MultiplyWithRoot" null null))
    (`KismetArrayLibrary.Array_Add` (`self.BoatArray`) _returnvalue))
  (bind _assailboat_controler (cast `/Game/BP/SailboatControler` (`GameplayStatics.GetPlayerController` 0)))
  (`Controller.Possess` _assailboat_controler (`|GetArrayItem` (`self.BoatArray`))))

(fn `UserConstructionScript`)