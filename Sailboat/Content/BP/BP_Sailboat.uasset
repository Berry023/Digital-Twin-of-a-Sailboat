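; Player-controlled sailboat with physics-based sailing, a three-step reefable mainsail, a left/right/rolled jib and an orbit camera.
; Each tick it derives apparent wind from the level's WindDirectionalSource and hull velocity, then applies angle-of-attack lift and drag for sails and keel.
; The rudder adds speed-squared yaw torque and drag, and self-centers faster at higher speed.
; The boom is either rotated manually or swings automatically with apparent wind, limited by player-controlled sail release.
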(event `InputAxis|Rudder Axis`
  (params (AxisValue :type "Float (single-precision)"))
  (`self.UpdateRudderInput` AxisValue (stale `self.ReceiveTick` DeltaSeconds))
  (`SceneComponent.K2_SetRelativeRotation` (`self.rudder`) (`KismetMathLibrary.MakeRotator` 0.0 0.0 (`self.RudderInput`)) false false))

(event `InputAction|Jib Left`
  (params (Key :type "Key Structure"))
  (bind _jib (`self.jib`))
  ;[1 1 1] Jib Left/Right positioning and rolled jib control
  (:`Pressed`
    (`SceneComponent.K2_SetRelativeRotation` _jib (struct :`Yaw` 10.0 :`Roll` -4.0) false false)
    (`SceneComponent.SetVisibility` _jib true false :!label _label)
    (`SceneComponent.SetVisibility` (`self.rolled_jib`) false false)
    (set `self.FrontSailArea` 25.0)))

(event `InputAxis|Look left/right`
  (params (AxisValue :type "Float (single-precision)"))
  ;[1 1 1] 360 camera movement (CameraBoom)
  (`self.AddControllerYawInput` AxisValue))

(event `self.ReceiveTick`
  (params (DeltaSeconds :type "Float (single-precision)"))
  (`self.UpdateSailForces`)
  (`self.RudderForces` (`self.RudderInput`) (`SceneComponent.GetComponentVelocity` (`self.hull`)))
  (`self.UpdateKeelForces`)
  (if (`self.IsBoomAuto`)
    (`self.Update Boom Rotation` DeltaSeconds)))

(event `InputAction|Jib Right`
  (params (Key :type "Key Structure"))
  ;[1 1 1] Jib Left/Right positioning and rolled jib control
  (:`Pressed`
    (`SceneComponent.K2_SetRelativeRotation` (`self.jib`) (struct :`Yaw` -10.0 :`Roll` 4.0) false false)
    (goto _label)))

(event `InputAxis|Look up/down`
  (params (AxisValue :type "Float (single-precision)"))
  ;[1 1 1] 360 camera movement (CameraBoom)
  (`self.AddControllerPitchInput` AxisValue))

(event `InputAction|Rolled Jib`
  (params (Key :type "Key Structure"))
  ;[1 1 1] Jib Left/Right positioning and rolled jib control
  (:`Pressed`
    (`SceneComponent.SetVisibility` (`self.jib`) false false)
    (`SceneComponent.SetVisibility` (`self.rolled_jib`) true false)
    (set `self.FrontSailArea` 0.0)))

(event `InputAxis|Boom Axis`
  (params (AxisValue :type "Float (single-precision)"))
  (bind _boom (`self.boom`))
  (bind (_relativerotation_roll _relativerotation_pitch _relativerotation_yaw) (`KismetMathLibrary.BreakRotator` (`SceneComponent.RelativeRotation` _boom)))
  (if (`self.IsBoomAuto`)
    (`self.UpdateSailRelease` AxisValue (stale `self.ReceiveTick` DeltaSeconds))
    (else
      (`SceneComponent.K2_SetRelativeRotation` _boom (`KismetMathLibrary.MakeRotator` 0.0 0.0 (`KismetMathLibrary.FClamp` (+ _relativerotation_yaw (* AxisValue 1.5)) -75.0 75.0)) false false))))

(event `InputAction|Main Sail State`
  (params (Key :type "Key Structure"))
  ;[1 1 1] Main Sail Full/Middle/Low Rotation
  (:`Pressed`
    (if (`self.MainSailGoingDown`)
      (set `self.MainSailStateIndex` (+ (`self.MainSailStateIndex`) 1))
      (if (== (`self.MainSailStateIndex`) 2)
        (set `self.MainSailGoingDown` false))
      (else
        (set `self.MainSailStateIndex` (- (`self.MainSailStateIndex`) 1))
        (if (== (`self.MainSailStateIndex`) 0)
          (set `self.MainSailGoingDown` true))))
    (switch `int` (`self.MainSailStateIndex`)
      (:`0`
        (`SceneComponent.SetVisibility` (`self.main_sail_full`) true false)
        (`SceneComponent.SetVisibility` (`self.main_sail_middle`) false false)
        (`SceneComponent.SetVisibility` (`self.main_sail_low`) false false)
        (set `self.MainSailArea` 50.0))
      (:`1`
        (`SceneComponent.SetVisibility` (`self.main_sail_full`) false false)
        (`SceneComponent.SetVisibility` (`self.main_sail_middle`) true false)
        (`SceneComponent.SetVisibility` (`self.main_sail_low`) false false)
        (set `self.MainSailArea` 35.0))
      (:`2`
        (`SceneComponent.SetVisibility` (`self.main_sail_full`) false false)
        (`SceneComponent.SetVisibility` (`self.main_sail_middle`) false false)
        (`SceneComponent.SetVisibility` (`self.main_sail_low`) true false)
        (set `self.MainSailArea` 20.0)))))

(event `self.ReceiveBeginPlay`
  (`WidgetBlueprintLibrary.SetInputMode_GameOnly` (`GameplayStatics.GetPlayerController` 0))
  (bind _outactors (`GameplayStatics.GetAllActorsOfClass` "/Script/Engine.WindDirectionalSource"))
  (set `self.WindActor` (`|GetArrayItem` _outactors))
  (`SceneComponent.SetVisibility` (`self.jib`) false false)
  (`SceneComponent.SetVisibility` (`self.rolled_jib`) true false)
  (`SceneComponent.SetVisibility` (`self.main_sail_full`) true false)
  (`SceneComponent.SetVisibility` (`self.main_sail_middle`) false false)
  (`SceneComponent.SetVisibility` (`self.main_sail_low`) false false))

(fn `CalculateAngleOfAttack`
  (params (ApparentWind :type "Vector Structure") (SailComponent :type "SceneComponent Object Reference"))
  (returns (AngleDeg :type "Float (double-precision)"))
  (bind _returnvalue (`KismetMathLibrary.Normal` ApparentWind))
  (bind _returnvalue_2 (`KismetMathLibrary.Normal` (`SceneComponent.GetForwardVector` SailComponent)))
  (return (* (`KismetMathLibrary.DegAcos` (`KismetMathLibrary.Dot_VectorVector` _returnvalue _returnvalue_2)) (`KismetMathLibrary.SignOfFloat` (`KismetMathLibrary.Dot_VectorVector` (`KismetMathLibrary.Cross_VectorVector` _returnvalue_2 _returnvalue) (`KismetMathLibrary.GetUpVector` (struct :`Yaw` 1.0)))))))

(fn `CalculateApparentWind`
  (params (TrueWind :type "Vector Structure"))
  (returns (ApparentWind :type "Vector Structure"))
  (return (- TrueWind (`SceneComponent.GetComponentVelocity` (`self.hull`)))))

(fn `CalculateDrag`
  (params (ApparentWind :type "Vector Structure") (AngleDeg :type "Float (double-precision)") (SailArea :type "Float (double-precision)"))
  (returns (Drag :type "Vector Structure"))
  (bind _returnvalue (`KismetMathLibrary.Cos` (`KismetMathLibrary.DegreesToRadians` AngleDeg)))
  (return (* (* (`KismetMathLibrary.Normal` ApparentWind) -1.0) (* (`KismetMathLibrary.VSizeSquared` ApparentWind) SailArea (* _returnvalue _returnvalue) (`self.AirDensity`) 0.5))))

(fn `CalculateKeelAngleOfAttack`
  (params (`Boat Velocity` :type "Vector Structure"))
  (returns (`Keel Angle Deg` :type "Float (double-precision)"))
  (bind _returnvalue (`KismetMathLibrary.Normal` `Boat Velocity`))
  (bind _returnvalue_2 (`KismetMathLibrary.Normal` (`self.GetActorForwardVector`)))
  (return (* (`KismetMathLibrary.DegAcos` (`KismetMathLibrary.Dot_VectorVector` _returnvalue _returnvalue_2)) (`KismetMathLibrary.SignOfFloat` (.z (`KismetMathLibrary.Cross_VectorVector` _returnvalue_2 _returnvalue))))))

(fn `CalculateKeelLiftAndDrag`
  (params (`Boat Velocity` :type "Vector Structure") (`Keel Angle Deg` :type "Float (double-precision)"))
  (returns (`Keel Lift Vector` :type "Vector Structure") (`Keel Drag Vector` :type "Vector Structure"))
  (bind _returnvalue (`KismetMathLibrary.Normal` `Boat Velocity`))
  (bind _returnvalue_2 (`KismetMathLibrary.DegreesToRadians` `Keel Angle Deg`))
  (bind _waterdensity (`self.WaterDensity`))
  (bind _keelarea (`self.KeelArea`))
  (bind _returnvalue_3 (`KismetMathLibrary.Square` (`KismetMathLibrary.VSize` `Boat Velocity`)))
  (return (* (`KismetMathLibrary.Cross_VectorVector` _returnvalue (`KismetMathLibrary.MakeVector` 0.0 0.0 1.0)) (* 0.5 _waterdensity _keelarea (`KismetMathLibrary.Sin` (* _returnvalue_2 2.0)) _returnvalue_3)) (* (* _returnvalue -1.0) (* 0.5 _waterdensity _keelarea (`KismetMathLibrary.Square` (`KismetMathLibrary.Cos` _returnvalue_2)) _returnvalue_3))))

(fn `CalculateLift`
  (params (ApparentWind :type "Vector Structure") (AngleDeg :type "Float (double-precision)") (SailArea :type "Float (double-precision)"))
  (returns (Lift :type "Vector Structure"))
  (bind _returnvalue (`KismetMathLibrary.Normal` ApparentWind))
  (return (* (`KismetMathLibrary.Cross_VectorVector` _returnvalue (`KismetMathLibrary.Cross_VectorVector` _returnvalue (`KismetMathLibrary.MakeVector` 0.0 0.0 1.0))) (* (* (`KismetMathLibrary.Sin` (* (`KismetMathLibrary.DegreesToRadians` AngleDeg) 2.0)) (* SailArea (`KismetMathLibrary.VSizeSquared` ApparentWind))) (`self.AirDensity`)))))

(fn `CalculateTrueWind`
  (returns (TrueWind :type "Vector Structure"))
  (bind _outactors (`GameplayStatics.GetAllActorsOfClass` "/Script/Engine.WindDirectionalSource"))
  (bind _returnvalue (`self.GetComponentByClass` (`|GetArrayItem` _outactors) "/Script/Engine.WindDirectionalSourceComponent"))
  (bind _output_get (set `self.WindSpeed` (`WindDirectionalSourceComponent.Strength` _returnvalue)))
  (bind _output_get_2 (set `self.WindDirection` (`KismetMathLibrary.GetForwardVector` (`SceneComponent.K2_GetComponentRotation` _returnvalue))))
  (return (* _output_get_2 _output_get)))

(fn `RudderForces`
  (params (RudderAngle :type "Float (double-precision)") (BoatVelocity :type "Vector Structure"))
  (bind _returnvalue (`KismetMathLibrary.VSizeSquared` BoatVelocity))
  (bind _returnvalue_2 (`KismetMathLibrary.DegreesToRadians` RudderAngle))
  (bind _waterdensity (`self.WaterDensity`))
  (bind _rudderarea (`self.RudderArea`))
  (bind _hull (`self.hull`))
  (`PrimitiveComponent.AddTorqueInRadians` _hull (`KismetMathLibrary.MakeVector` 0.0 0.0 (* (* 0.5 _waterdensity _rudderarea _returnvalue (`KismetMathLibrary.Sin` (* 2.0 _returnvalue_2))) (`self.DistanceToRudder`))) "None" false)
  (`PrimitiveComponent.AddForce` _hull (* (* 0.5 _waterdensity _rudderarea _returnvalue (`KismetMathLibrary.Square` (`KismetMathLibrary.Cos` _returnvalue_2))) (* (`KismetMathLibrary.Normal` (`KismetMathLibrary.MakeVector` (.x BoatVelocity) (.y BoatVelocity))) -1.0) 0.0001) "None" false))

(fn `Update Boom Rotation`
  (params (`Delta Time` :type "Float (double-precision)"))
  (bind _returnvalue (* (`self.SailRelease`) (`self.MaxSailAngle`)))
  (bind (_relativerotation_roll _relativerotation_pitch _relativerotation_yaw) (`KismetMathLibrary.BreakRotator` (`SceneComponent.RelativeRotation` (`self.boom`))))
  (bind _truewind (`self.CalculateTrueWind`))
  (bind _apparentwind (`self.CalculateApparentWind` _truewind))
  (bind (_returnvalue_roll _returnvalue_pitch _returnvalue_yaw) (`KismetMathLibrary.BreakRotator` (`KismetMathLibrary.FindLookAtRotation` (`KismetMathLibrary.Normal` (`KismetMathLibrary.MakeVector` (.x (`self.GetActorForwardVector`)) (.y (`self.GetActorForwardVector`)))) (`KismetMathLibrary.Normal` (`KismetMathLibrary.MakeVector` (.x _apparentwind) (.y _apparentwind))))))
  (`SceneComponent.K2_SetRelativeRotation` (`self.boom`) (`KismetMathLibrary.MakeRotator` 0.0 0.0 (`KismetMathLibrary.FInterpTo` _relativerotation_yaw (`KismetMathLibrary.FClamp` _returnvalue_yaw (* _returnvalue -1.0) _returnvalue) `Delta Time` (* (`KismetMathLibrary.VSize` _apparentwind) 0.03))) false false))

(fn `UpdateKeelForces`
  (bind _returnvalue (`SceneComponent.GetComponentVelocity` (`self.hull`)))
  (bind _keel_angle_deg (`self.CalculateKeelAngleOfAttack` _returnvalue))
  (bind (_keel_lift_vector _keel_drag_vector) (`self.CalculateKeelLiftAndDrag` _returnvalue _keel_angle_deg))
  (`PhysicsThreadLibrary.AddForce` (struct) (+ _keel_lift_vector _keel_drag_vector)))

(fn `UpdateRudderInput`
  (params (AxisValue :type "Float (double-precision)") (`Delta Time` :type "Float (double-precision)"))
  (bind _maxrudderangle (`self.MaxRudderAngle`))
  (bind _maxrudderangle_2 (`self.MaxRudderAngle`))
  (bind _maxrudderangle_3 (`self.MaxRudderAngle`))
  (bind _returnvalue (* (+ (* (`KismetMathLibrary.VSize` (`SceneComponent.GetComponentVelocity` (`self.hull`))) (`self.ReturnSpeedMultiplier`)) (`self.BaseRotationSpeed`)) `Delta Time`))
  (bind _returnvalue_2 (+ (`self.RudderInput`) _returnvalue))
  (bind _returnvalue_3 (- (`self.RudderInput`) _returnvalue))
  (if (== AxisValue 0.0)
    (if (> (`self.RudderInput`) 0.0)
      (if (< (`KismetMathLibrary.Abs` _returnvalue_3) 1.0)
        (set `self.RudderInput` 0.0)
        (else
          (set `self.RudderInput` (`KismetMathLibrary.FClamp` _returnvalue_3 (* -1.0 _maxrudderangle_3) _maxrudderangle_3))))
      (elif (< (`KismetMathLibrary.Abs` _returnvalue_2) 1.0)
        (set `self.RudderInput` 0.0)
        (else
          (set `self.RudderInput` (`KismetMathLibrary.FClamp` _returnvalue_2 (* -1.0 _maxrudderangle_2) _maxrudderangle_2)))))
    (else
      (set `self.RudderInput` (`KismetMathLibrary.FClamp` (+ (* AxisValue `Delta Time` (`self.RudderRotationSpeed`)) (`self.RudderInput`)) (* -1.0 _maxrudderangle) _maxrudderangle)))))

(fn `UpdateSailForces`
  (bind _mainsailarea (`self.MainSailArea`))
  (bind _frontsailarea (`self.FrontSailArea`))
  (bind _mainsailarea_2 (`self.MainSailArea`))
  (bind _frontsailarea_2 (`self.FrontSailArea`))
  (bind _mainsailarea_3 (`self.MainSailArea`))
  (bind _frontsailarea_3 (`self.FrontSailArea`))
  (bind _truewind (`self.CalculateTrueWind`))
  (bind _apparentwind (`self.CalculateApparentWind` _truewind))
  (switch `int` (`self.MainSailStateIndex`)
    (:`0`
      (bind _angledeg (`self.CalculateAngleOfAttack` _apparentwind (`self.main_sail_full`)))
      (bind _angledeg_2 (`self.CalculateAngleOfAttack` _apparentwind (`self.jib`)))
      (bind _lift (`self.CalculateLift` _apparentwind _angledeg _mainsailarea_3))
      (bind _lift_2 (`self.CalculateLift` _apparentwind _angledeg_2 _frontsailarea_3))
      (bind _drag (`self.CalculateDrag` _apparentwind _angledeg _mainsailarea_3))
      (bind _drag_2 (`self.CalculateDrag` _apparentwind _angledeg_2 _frontsailarea_3))
      (`PrimitiveComponent.AddForce` (`self.hull`) (* (+ (+ _lift _drag) (+ _lift_2 _drag_2)) 0.1) "None" false))
    (:`1`
      (bind _angledeg_3 (`self.CalculateAngleOfAttack` _apparentwind (`self.main_sail_middle`)))
      (bind _angledeg_4 (`self.CalculateAngleOfAttack` _apparentwind (`self.jib`)))
      (bind _lift_3 (`self.CalculateLift` _apparentwind _angledeg_3 _mainsailarea))
      (bind _lift_4 (`self.CalculateLift` _apparentwind _angledeg_4 _frontsailarea))
      (bind _drag_3 (`self.CalculateDrag` _apparentwind _angledeg_3 _mainsailarea))
      (bind _drag_4 (`self.CalculateDrag` _apparentwind _angledeg_4 _frontsailarea))
      (`PrimitiveComponent.AddForce` (`self.hull`) (+ (+ _lift_3 _drag_3) (+ _lift_4 _drag_4)) "None" false))
    (:`2`
      (bind _angledeg_5 (`self.CalculateAngleOfAttack` _apparentwind (`self.main_sail_low`)))
      (bind _angledeg_6 (`self.CalculateAngleOfAttack` _apparentwind (`self.jib`)))
      (bind _lift_5 (`self.CalculateLift` _apparentwind _angledeg_5 _mainsailarea_2))
      (bind _lift_6 (`self.CalculateLift` _apparentwind _angledeg_6 _frontsailarea_2))
      (bind _drag_5 (`self.CalculateDrag` _apparentwind _angledeg_5 _mainsailarea_2))
      (bind _drag_6 (`self.CalculateDrag` _apparentwind _angledeg_6 _frontsailarea_2))
      (`PrimitiveComponent.AddForce` (`self.hull`) (+ (+ _lift_5 _drag_5) (+ _lift_6 _drag_6)) "None" false))))

(fn `UpdateSailRelease`
  (params (`Axis Value` :type "Float (double-precision)") (`Delta Time` :type "Float (double-precision)"))
  (set `self.SailRelease` (`KismetMathLibrary.FClamp` (+ (* `Axis Value` `Delta Time` (`self.BoomReleaseSpeed`)) (`self.SailRelease`)))))

(fn `UserConstructionScript`)